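; WorldClickLibrary is a Blueprint function library that handles a right click on the world at a screen location.
; TryRightClickWorld deprojects the screen point and runs a Visibility line trace along that ray, with debug drawing left on.
; An Interactable hit spawns its interact GUI for the Interactor, while any other hit moves the controller to the impact point with SimpleMoveToLocation.
; It returns success with the hit, or failure when deprojection or the trace fails.
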(fn TryRightClickWorld
  (params (PlayerController :type Player%20Controller%20Object%20Reference) (Interactor :type Actor%20Object%20Reference) (ScreenLocation :type Vector%202D%20Structure))
  (bind (_worldposition _worlddirection _returnvalue) (Class|GameplayStatics|DeprojectScreentoWorld PlayerController ScreenLocation))
  ;[1 1 1] Deproject Screen
  (if _returnvalue
    ;[1 1 1] Interactable Hit?
    (bind (_outhit _returnvalue_2) (Collision|LineTraceByChannel 0 _worldposition (+ _worldposition (* _worlddirection 1e+04)) "TraceTypeQuery1" false 0 "ForDuration" true "(R=1.000000,G=0.248636,B=0.000000,A=1.000000)" "(R=0.000000,G=1.000000,B=0.000000,A=1.000000)" 2.0))
    (if _returnvalue_2
      (bind _asinteractable (Utilities|Casting|CastToInteractable (.HitActor (Collision|BreakHitResult _outhit)))
        (:then
          ;[1 1 1] Interactable Hit
          (Class|Interactable|SpawnInteractGUI _asinteractable Interactor)
          (return true _outhit))
        (:CastFailed
          ;[1 1 1] Interactable Not Hit
          (AI|Navigation|SimpleMovetoLocation PlayerController (.ImpactPoint (Collision|BreakHitResult _outhit)))
          (return true _outhit)))
      (else
        _)))
  ;[1 1 1] Failure
  (return false ""))